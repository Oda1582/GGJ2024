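; Player Blueprint that manages health, a level countdown, the HUD, and the pause and death menus.
; Tick counts down the level duration and prints a win message once at zero.
; AnyDamage adds the damage value to health, so only negative values hurt; it caps at max like Heal and calls GameOver at zero.
; Escape or P opens the pause menu and pauses the game, while GameOver shows the death menu without pausing.
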(event `self.ReceiveTick`
  (params (DeltaSeconds :type "Float (single-precision)"))
  ;[1 0.5391 0] Handle Level Duration
  (set `self.LevelDuration` (- (`self.LevelDuration`) DeltaSeconds))
  (if (<= (`self.LevelDuration`) 0.0)
    (`/Engine/EditorBlueprintResources/StandardMacros.DoOnce` false
      (:`Completed`
        (`KismetSystemLibrary.PrintString` "You Won")))))

(event `self.ReceiveBeginPlay`
  ;[0 1 0.3672] Set Max Health
  (set `self.Health` (`self.HealthMax`))
  ;[0.1953 1 0] Add HUD to screen
  (bind _returnvalue (`|CreateWidget` "/Game/BP/HUD/WBP_InfoPlayer.WBP_InfoPlayer_C"))
  (bind _output_get (set `self.HUDRef` _returnvalue))
  (`UserWidget.AddToViewport` _output_get 0)
  (set `self.LevelDuration` (`self.LevelDurationMax`)))

(event `self.ReceiveAnyDamage`
  (params (Damage :type "Float (single-precision)") (DamageType :type "DamageType Object Reference") (InstigatedBy :type "Controller Object Reference") (DamageCauser :type "Actor Object Reference"))
  ;[0 0.2734 1] Check Health
  (`KismetSystemLibrary.PrintString` "You get damage")
  (set `self.Health` (+ (`self.Health`) Damage))
  (`|ExecutionSequence`
    (:`then_0`
      ;;[0 1 0.01562] Check if under 0 health
      (if (<= (`self.Health`) 0.0)
        (`KismetSystemLibrary.PrintString` "You're Dead")
        (`self.Game Over`)))
    (:`then_1`
      ;;[1 0 0.9609] Check if higher than max health
      (if (>= (`self.Health`) (`self.HealthMax`))
        (set `self.Health` (`self.HealthMax`))))))

(event `Key|Escape`
  (params (Key :type "Key Structure"))
  (bind _returnvalue (`GameplayStatics.GetPlayerController` 0))
  ;[1 0 0.4453] Pour le MenuPause
  (:`Pressed`
    (if (not (`self.isPauseMenuOpened?`)) :!label _label
      (`WidgetBlueprintLibrary.SetInputMode_UIOnlyEx` _returnvalue null "DoNotLock" true)
      (set `PlayerController.bShowMouseCursor` true _returnvalue)
      (bind _returnvalue_2 (`|CreateWidget` "/Game/BP/HUD/WBP_PauseMenu.WBP_PauseMenu_C"))
      (bind _output_get (set `self.UIMenuPause` _returnvalue_2))
      (`UserWidget.AddToViewport` _output_get 0)
      (set `self.isPauseMenuOpened?` true)
      (`GameplayStatics.SetGamePaused` true))))

(event `Key|P`
  (params (Key :type "Key Structure"))
  ;[1 0 0.4453] Pour le MenuPause
  (:`Pressed`
    (goto _label)))

(fn `Game Over`
  (bind _returnvalue (`GameplayStatics.GetPlayerController` 0))
  ;[1 0 0.07031] Add Death HUD
  (`KismetSystemLibrary.PrintString` "Game Over")
  (`WidgetBlueprintLibrary.SetInputMode_UIOnlyEx` _returnvalue null "DoNotLock" true)
  (set `PlayerController.bShowMouseCursor` true _returnvalue)
  (bind _returnvalue_2 (`|CreateWidget` "/Game/BP/HUD/WBP_MortMenu.WBP_MortMenu_C"))
  (bind _output_get (set `self.UIMortMenu` _returnvalue_2))
  (`UserWidget.AddToViewport` _output_get 0))

(fn `Heal`
  (params (`Heal Value` :type "Float (double-precision)"))
  (`KismetSystemLibrary.PrintString` "Heal")
  (set `self.Health` (+ (`self.Health`) `Heal Value`))
  (if (>= (`self.Health`) (`self.HealthMax`))
    (set `self.Health` (`self.HealthMax`))))

(fn `UserConstructionScript`)