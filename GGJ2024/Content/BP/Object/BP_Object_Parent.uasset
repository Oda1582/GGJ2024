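; Base class for clickable household objects that affect the player, killer and baby, configured from a DT_Object row.
; Clicking a usable object damages the player, reports noise to the killer, adjusts baby happiness by reaction-type match and plays its sound.
; Use starts a Tick-driven cooldown shown by a widget, with the point light signalling availability.
; Hovering swaps in a highlight material and reveals the name text, which is oriented toward the camera on BeginPlay.
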(event `self.ReceiveBeginPlay`
  (bind _object_properties_objectname (break `/Game/Data_Table/DS_Object` (`self.Object Properties`)))
  (bind _object_name (`self.Object Name`))
  (`|ExecutionSequence`
    (:`then_0`
      ;[1 0.5859 0] References
      (bind _asbp_player (cast `/Game/BP/BP_Player` (`GameplayStatics.GetPlayerPawn` 0)))
      (set `self.As BP Player` _asbp_player)
      (bind _returnvalue (`GameplayStatics.GetActorOfClass` "/Game/BP/BP_Killer.BP_Killer_C"))
      (set `self.KillerRef` _returnvalue)
      (bind _returnvalue_2 (`GameplayStatics.GetActorOfClass` "/Game/BP/BP_Baby.BP_Baby_C"))
      (set `self.BabyRef` _returnvalue_2))
    (:`then_1`
      ;[0 0.8359 1] Object Properties
      (bind _returnvalue_3 (`|GetDataTableRow` "/Game/Data_Table/DT_Object.DT_Object" (`self.DT_Object`))
        (:`then`
          (bind _output_get (set `self.Object Properties` _returnvalue_3))
          (bind _output_get_2 (set `self.Object_Cooldown` (`.Cooldown_27_9300EE5042EF97E061633F80B5E0B542` (break `/Game/Data_Table/DS_Object` _output_get))))
          (set `self.Object_MaxCooldown` _output_get_2)
          ;[0.3359 1 0] Save Original Material as a variable
          (set `self.OG Material Index0` (`PrimitiveComponent.GetMaterial` (`self.Object`) 0))
          (set `self.OG Material Index1` (`PrimitiveComponent.GetMaterial` (`self.Object`) 1))
          ;[1 0 0.8672] Hide Text
          (`SceneComponent.SetVisibility` (`self.Object Name`) false false)
          ;[1 0 0.3047] Set Name Text
          (`TextRenderComponent.K2_SetText` (`self.Object Name`) (`KismetTextLibrary.Conv_StringToText` _object_properties_objectname))
          ;[0.6406 1 0] Put Light visible
          (`SceneComponent.SetVisibility` (`self.PointLight`) true false)
          ;[0 0.7187 1] Orient text to cam
          (`SceneComponent.K2_SetWorldRotation` _object_name (`KismetMathLibrary.FindLookAtRotation` (`SceneComponent.K2_GetComponentLocation` _object_name) (`SceneComponent.K2_GetComponentLocation` (`/Game/BP/BP_Player.Camera` (`self.As BP Player`)))) false false))))
    (:`then_2`
      ;[1 0 0.4453] HUD
      (`SceneComponent.SetVisibility` (`self.Cooldown`) false false)
      (bind _returnvalue_4 (`|CreateWidget` "/Game/BP/HUD/WBP_Cooldown.WBP_Cooldown_C"))
      (set `self.CooldownRef` _returnvalue_4)
      (`WidgetComponent.SetWidget` (`self.Cooldown`) _returnvalue_4))))

(event `self.ReceiveTick`
  (params (DeltaSeconds :type "Float (single-precision)"))
  (bind (_object_properties_objectname _object_properties_noise_lvl _object_properties_damage _object_properties_basehappiness _object_properties_happinessbuff _object_properties_happinessdebuff _object_properties_cooldown) (break `/Game/Data_Table/DS_Object` (`self.Object Properties`)))
  ;[0.03125 0 1] Starts cooldown if used
  (if (not (`self.Useable`))
    ;[0.5469 1 0] Cooldown
    (bind _output_get (set `self.Object_Cooldown` (- (`self.Object_Cooldown`) DeltaSeconds)))
    (`/Game/BP/HUD/WBP_Cooldown.CoolDownFunctionV2` (`self.CooldownRef`) _output_get (`self.Object_MaxCooldown`))
    ;[0.6641 1 0] Check if Cooldown is done
    (if (<= (`self.Object_Cooldown`) 0.0)
      ;[0.6406 1 0] Make Object useable again
      (set `self.Useable` true)
      (set `self.Object_Cooldown` _object_properties_cooldown)
      (`KismetSystemLibrary.PrintString` "Is Useable Again")
      (`SceneComponent.SetVisibility` (`self.PointLight`) true false)
      (`SceneComponent.SetVisibility` (`self.Cooldown`) false false))))

(event `self.Object.OnClicked`
  (params (TouchedComponent :type "PrimitiveComponent Object Reference") (ButtonPressed :type "Key Structure"))
  (bind (_object_properties_objectname _object_properties_noise_lvl _object_properties_damage _object_properties_basehappiness _object_properties_happinessbuff _object_properties_happinessdebuff _object_properties_cooldown _object_properties_reactiontype _object_properties_objectsound) (break `/Game/Data_Table/DS_Object` (`self.Object Properties`)))
  (bind (_objectname _noise_lvl _damage) (break `/Game/Data_Table/DS_Object` (`self.Object Properties`)))
  ;[1 0.3281 0] Set in Used when clicked on
  (if (`self.Useable`)
    (set `self.Useable` false)
    ;[0.125 1 0] Deactivate Light and Activate HUD
    (`SceneComponent.SetVisibility` (`self.PointLight`) false false)
    (`SceneComponent.SetVisibility` (`self.Cooldown`) true false)
    ;[0 1 0.4844] Give Damage according to Object properties
    (`GameplayStatics.ApplyDamage` (`self.As BP Player`) _damage)
    ;[1 0 0.5859] Add Noises
    (`/Game/BP/BP_Killer.Check_NoiseLVL` (`self.KillerRef`) _noise_lvl)
    ;[0 1 0.7656] Give or lose happiness according to the reaction type
    (`self.CheckIfMatchingReactionObject`)
    ;[0.1719 0 1] Play Object Sound
    (bind _returnvalue (`GameplayStatics.SpawnSound2D` _object_properties_objectsound 1.0 1.0 0.0 null))
    (bind _output_get (set `self.ObjectsUseSound` _returnvalue))
    (`/Engine/EditorBlueprintResources/StandardMacros.IsValid` _output_get
      (:`Is Valid`
        (if (`AudioComponent.IsPlaying` _output_get)
          (`AudioComponent.Stop` (`self.ObjectsUseSound`)))
        (`AudioComponent.Play` (`self.ObjectsUseSound`) 0.0)))))

(event `self.Collision_Mesh.OnClicked`
  (params (TouchedComponent :type "PrimitiveComponent Object Reference") (ButtonPressed :type "Key Structure")))

(event `self.Collision_Mesh.OnBeginCursorOver`
  (params (TouchedComponent :type "PrimitiveComponent Object Reference"))
  ;[1 0 0.7969] Change Collision with mouse on it or not
)

(event `self.Object.OnBeginCursorOver`
  (params (TouchedComponent :type "PrimitiveComponent Object Reference"))
  ;[1 0 0.7969] Change Collision with mouse on it or not
  (`PrimitiveComponent.SetMaterial` (`self.Object`) 0 "/Game/Material/M_Highlight.M_Highlight")
  (`PrimitiveComponent.SetMaterial` (`self.Object`) 1 "/Game/Material/M_Highlight.M_Highlight")
  (`SceneComponent.SetVisibility` (`self.Object Name`) true false))

(event `self.Collision_Mesh.OnEndCursorOver`
  (params (TouchedComponent :type "PrimitiveComponent Object Reference"))
  ;[1 0 0.7969] Change Collision with mouse on it or not
)

(event `self.Object.OnEndCursorOver`
  (params (TouchedComponent :type "PrimitiveComponent Object Reference"))
  ;[1 0 0.7969] Change Collision with mouse on it or not
  (`PrimitiveComponent.SetMaterial` (`self.Object`) 0 (`self.OG Material Index0`))
  (`PrimitiveComponent.SetMaterial` (`self.Object`) 1 (`self.OG Material Index1`))
  (`SceneComponent.SetVisibility` (`self.Object Name`) false false))

(fn `CheckIfMatchingReactionObject`
  (bind (_object_properties_objectname _object_properties_noise_lvl _object_properties_damage _object_properties_basehappiness _object_properties_happinessbuff _object_properties_happinessdebuff _object_properties_cooldown _object_properties_reactiontype) (break `/Game/Data_Table/DS_Object` (`self.Object Properties`)))
  (`/Game/BP/BP_Baby.Gain/Lose Happiness` (`self.BabyRef`) _object_properties_basehappiness _object_properties_happinessbuff _object_properties_happinessdebuff (`|EnumEquality` (`/Game/BP/BP_Baby.ReactionType` (`self.BabyRef`)) _object_properties_reactiontype)))

(fn `MakeUseable`
  (params (Useable :type Boolean))
  (`SceneComponent.SetVisibility` (`self.PointLight`) Useable false))

(fn `UserConstructionScript`)