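; Baby actor whose happiness drains every tick and drives how fast the killer's awareness rises.
; Happiness thresholds select one of five reactions, from crying to hysterical laughter, each change refreshing the emoji widget and playing a 2D sound.
; All but normal laughter set BP_Killer's awareness rate, with hysterical laughter the highest.
; GainLoseHappiness applies clamped changes, adjusted by object-reaction matching while the baby is reacting.
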(event `self.ReceiveBeginPlay`
  ;[1 0.1875 0] References
  (bind _returnvalue (`GameplayStatics.GetActorOfClass` "/Game/BP/BP_Killer.BP_Killer_C"))
  (set `self.Killer Ref` _returnvalue)
  (bind _returnvalue_2 (`|CreateWidget` "/Game/BP/HUD/WBP_Baby_Emoji.WBP_Baby_Emoji_C"))
  (bind _output_get (set `self.EmojiRef` _returnvalue_2))
  (`WidgetComponent.SetWidget` (`self.Emoji HUD`) _output_get)
  (`/Game/BP/HUD/WBP_Baby_Emoji.Show Emoji` (`self.EmojiRef`))
  (bind _outactors (`GameplayStatics.GetAllActorsOfClass` "/Game/BP/Object/BP_Object_Parent.BP_Object_Parent_C"))
  (set `self.AllObject` _outactors))

(event `self.ReceiveTick`
  (params (DeltaSeconds :type "Float (single-precision)"))
  ;[0.7109 0 1] Baby Happiness Decrease constantly
  (if (> (`self.Baby Happiness`) 0.0)
    (set `self.Baby Happiness` (- (`self.Baby Happiness`) (* DeltaSeconds (`self.Baby Happiness Decrease Rate`))))
    ;[1 0.9375 0] Change la réaction du bébé en fonction de son happiness et augmente ou descend la rapidité d'augmentation de l'attention du tueur
    (if (<= (`self.Baby Happiness`) 10.0)
      (if (`|EnumInequality` (`self.ReactionType`) "NewEnumerator0")
        ;;[1 0 0.5391] Pleure
        (set `self.ReactionType` "NewEnumerator0")
        (set `/Game/BP/BP_Killer.Increase Awareness Rate` 3.0 (`self.Killer Ref`))
        ;[1 0 0.75] Show HUD and play sound
        (`/Game/BP/HUD/WBP_Baby_Emoji.Show Emoji` (`self.EmojiRef`) :!label _label)
        ;[1 0 0.3516] Play Sound and stop it if one is already playing
        (bind _returnvalue (`GameplayStatics.SpawnSound2D` (select `/Game/BP/Enum_BabyReaction` (`self.ReactionType`) :`NewEnumerator0` "/Game/Asset/Sons/Baby/Cry/SC_Cry.SC_Cry" :`NewEnumerator1` "/Game/Asset/Sons/Baby/Scream/SC_Baby_Scream.SC_Baby_Scream" :`NewEnumerator2` "/Game/Asset/Sons/Baby/Tantrum/SC_TapePartout.SC_TapePartout" :`NewEnumerator4` "/Game/Asset/Sons/Baby/Laugh/SC_BabyLaugh.SC_BabyLaugh" :`NewEnumerator5` "/Game/Asset/Sons/Baby/Big_Laugh/SC_Bebe_rigole.SC_Bebe_rigole" :!type "SoundBase Object Reference") 1.0 1.0 0.0 null))
        (bind _output_get (set `self.StatusReactionSound` _returnvalue))
        (`/Engine/EditorBlueprintResources/StandardMacros.IsValid` _output_get
          (:`Is Valid`
            (for _array_element (`self.AllObject`)
              (bind _canusesound (`/Game/BP/Object/BP_Object_Parent.Check if anynoise is happening` _array_element))
              (if _canusesound
                (break)))
            (if (`AudioComponent.IsPlaying` (`self.StatusReactionSound`))
              (`AudioComponent.Stop` (`self.StatusReactionSound`)))
            (`AudioComponent.Play` (`self.StatusReactionSound`) 0.0))))
      (elif (<= (`self.Baby Happiness`) 20.0)
        (if (`|EnumInequality` (`self.ReactionType`) "NewEnumerator1")
          ;;[0 0.6953 1] Cri
          (set `self.ReactionType` "NewEnumerator1")
          (set `/Game/BP/BP_Killer.Increase Awareness Rate` 2.5 (`self.Killer Ref`))
          (goto _label))
        (elif (<= (`self.Baby Happiness`) 30.0)
          (if (`|EnumInequality` (`self.ReactionType`) "NewEnumerator2")
            ;;[0.8516 0 1] Tape Partout
            (set `self.ReactionType` "NewEnumerator2")
            (set `/Game/BP/BP_Killer.Increase Awareness Rate` 2.0 (`self.Killer Ref`))
            (set `self.IsReacting` true)
            (goto _label))
          (elif (<= (`self.Baby Happiness`) 80.0)
            (if (`|EnumInequality` (`self.ReactionType`) "NewEnumerator4")
              (set `self.ReactionType` "NewEnumerator4")
              ;;[0.8516 0 1] Rire Normal
              (set `self.IsReacting` false)
              (goto _label))
            (elif (`|EnumInequality` (`self.ReactionType`) "NewEnumerator5")
              (set `self.ReactionType` "NewEnumerator5")
              ;;[0.2891 0 1] Rire Hystérique
              (set `/Game/BP/BP_Killer.Increase Awareness Rate` 4.0 (`self.Killer Ref`))
              (goto _label))))))))

(fn `Gain/Lose Happiness`
  (params (BaseHappiness :type "Float (double-precision)") (`Happiness Buff` :type "Float (double-precision)") (`Happiness Debuff` :type "Float (double-precision)") (Matching :type Boolean))
  ;[0.4766 1 0] Object reacts differently if he's reacting or not
  (if (`self.IsReacting`)
    ;[0 0.6016 1] Check if the object and the reaction is matching
    (if Matching
      ;[1 0 0.7031] Give Happiness Buff
      (set `self.Baby Happiness` (+ (`self.Baby Happiness`) (+ BaseHappiness `Happiness Buff`)))
      (`/Game/BP/HUD/WBP_Baby_Emoji.Show Matching Reaction` (`self.EmojiRef`))
      (else
        ;[1 0.2344 0] Give Less Happiness if wrong object
        (set `self.Baby Happiness` (+ (`self.Baby Happiness`) (- BaseHappiness `Happiness Debuff`)))
        (`/Game/BP/HUD/WBP_Baby_Emoji.Show Unmatched Reaction` (`self.EmojiRef`))))
    (else
      ;[1 0 0.7031] Give Happiness Buff
      (set `self.Baby Happiness` (+ (`self.Baby Happiness`) BaseHappiness))
      (`/Game/BP/HUD/WBP_Baby_Emoji.Show Base Reaction` (`self.EmojiRef`))))
  ;[1 0.07031 0] Set at the max if passed
  (`|ExecutionSequence`
    (:`then_0`
      (if (>= (`self.Baby Happiness`) (`self.Baby Max Happiness`))
        (set `self.Baby Happiness` (`self.Baby Max Happiness`))))
    (:`then_1`
      (if (<= (`self.Baby Happiness`) 0.0)
        (set `self.Baby Happiness` 0.0)))))

(fn `UserConstructionScript`)