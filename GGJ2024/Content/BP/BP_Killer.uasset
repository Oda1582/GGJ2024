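; Killer actor that tracks noise as an awareness level and ends the game through the player's GameOver when it reaches the maximum.
; Each Tick, awareness rises while the baby is reacting or its BabyHappiness is at least 80, and otherwise decays toward zero.
; CheckNoiseLVL adds incoming noise and checks the same limit.
; A point light's intensity is range-mapped from the current level as visual feedback.
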(event `self.ReceiveTick`
  (params (DeltaSeconds :type "Float (single-precision)"))
  ;[0.8047 0 1] Handles increase and decrease of noise level
  (if (and (> (`self.Noise_LvL`) 0.0) (not (`/Game/BP/BP_Baby.IsReacting` (`self.BabyRef`))))
    ;[1 0 0.1406] If the baby is not reacting and that you're noise lvl is above 0
    (if (not (>= (`/Game/BP/BP_Baby.Baby Happiness` (`self.BabyRef`)) 80.0))
      (set `self.Noise_LvL` (- (`self.Noise_LvL`) (* DeltaSeconds (`self.DecreaseAwarenessRate`))))
      (`self.Set Light Intensity based on noise`)
      ;[0.875 1 0] Die if reach the max awareness
      (if (>= (`self.Noise_LvL`) (`self.Noise_MaxLVL`)) :!label _label
        (`/Engine/EditorBlueprintResources/StandardMacros.DoOnce` false
          (:`Completed`
            (`/Game/BP/BP_Player.Game Over` (`self.As BP Player`)))))
      (else
        ;[1 0 0.1641] The awareness of the killer increase if the baby is reacting
        (if (or (`/Game/BP/BP_Baby.IsReacting` (`self.BabyRef`)) (>= (`/Game/BP/BP_Baby.Baby Happiness` (`self.BabyRef`)) 80.0)) :!label _label_2
          (set `self.Noise_LvL` (+ (`self.Noise_LvL`) (* DeltaSeconds (`self.Increase Awareness Rate`))))
          (`self.Set Light Intensity based on noise`)
          (goto _label))))
    (else
      (goto _label_2))))

(event `self.ReceiveBeginPlay`
  ;[0.1016 1 0] References
  (bind _asbp_player (cast `/Game/BP/BP_Player` (`GameplayStatics.GetPlayerPawn` 0)))
  (set `self.As BP Player` _asbp_player)
  (bind _returnvalue (`GameplayStatics.GetActorOfClass` "/Game/BP/BP_Baby.BP_Baby_C"))
  (set `self.BabyRef` _returnvalue))

(fn `Check_NoiseLVL`
  (params (NoiseReceived :type "Float (double-precision)"))
  (set `self.Noise_LvL` (+ NoiseReceived (`self.Noise_LvL`)))
  (bind _returnvalue (`self.Set Light Intensity based on noise`))
  (`KismetSystemLibrary.PrintString` (`KismetStringLibrary.Conv_DoubleToString` _returnvalue))
  (if (>= (`self.Noise_LvL`) (`self.Noise_MaxLVL`))
    (`/Game/BP/BP_Player.Game Over` (`self.As BP Player`))))

(fn `Set Light Intensity based on noise`
  (returns (ReturnValue :type "Float (double-precision)"))
  (bind _returnvalue (`KismetMathLibrary.MapRangeClamped` (`self.Noise_LvL`) 0.0 (`self.Noise_MaxLVL`) 0.0 50000.0))
  (`LightComponent.SetIntensity` (`self.PointLight`) _returnvalue)
  (return _returnvalue))

(fn `UserConstructionScript`)